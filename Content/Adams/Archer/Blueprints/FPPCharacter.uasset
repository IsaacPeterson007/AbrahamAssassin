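; First-person player character Blueprint that handles walking, sprinting, jumping and look control.
; Hardcoded WASD key events set forward and right axis values, which Tick applies as movement along control-rotation vectors while feeding raw axis-key values into pitch and yaw.
; BeginPlay tunes jump, gravity, air control and walk speed, and Left Shift swaps walk speed for sprinting.
; Input bypasses project action and axis mappings, which the graph's comments flag as unsuitable for a final build.
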(event EventBeginPlay
  (bind _charactermovement (Variables|Character|GetCharacterMovement))
  ;[1 1 1] Setting default parameters for player movement
  (Variables|/Script/Engine.CharacterMovementComponent|SetJumpZVelocity _charactermovement 8e+02)
  (Variables|/Script/Engine.CharacterMovementComponent|SetMaxWalkSpeed _charactermovement 9e+02)
  (Variables|/Script/Engine.CharacterMovementComponent|SetGravityScale _charactermovement 2.0)
  (Variables|/Script/Engine.CharacterMovementComponent|SetAirControl _charactermovement 1.0))

(event EventTick
  (params (DeltaSeconds :type Float%20%28single-precision%29))
  (bind _returnvalue (Pawn|GetControlRotation :!class /Script/Engine.Pawn))
  ;[1 1 1] Controlling player movement
  ;;[1 1 1] Applying movemnent
  (Pawn|Input|AddMovementInput (Math|Vector|GetForwardVector _returnvalue) (Variables|Default|GetforwardAxis) false)
  (Pawn|Input|AddMovementInput (Math|Vector|GetRightVector _returnvalue) (Variables|Default|GetrightAxis) false)
  ;[1 1 1] Controlling player rotation
  (Pawn|Input|AddControllerPitchInput (* (Class|Actor|GetInputAxisKeyValue) -1.0))
  (Pawn|Input|AddControllerYawInput (Class|Actor|GetInputAxisKeyValue)))

(event Input|KeyboardEvents|LeftShift
  (params (Key :type Key%20Structure))
  (bind _charactermovement (Variables|Character|GetCharacterMovement))
  ;[1 0.2708 0.2708] Please don't do this in your final build. Always use 'Edit > Project Settings > Input' to set up action and axis mappings.
  ;;[1 1 1] Make player run when Shift key is pressed
  (:Pressed
    (Variables|/Script/Engine.CharacterMovementComponent|SetMaxWalkSpeed _charactermovement 1.3e+03))
  (:Released
    (Variables|/Script/Engine.CharacterMovementComponent|SetMaxWalkSpeed _charactermovement 9e+02)))

(event Input|KeyboardEvents|W
  (params (Key :type Key%20Structure))
  ;[1 0.2708 0.2708] Please don't do this in your final build. Always use 'Edit > Project Settings > Input' to set up action and axis mappings.
  ;;[1 1 1] Assigning keys for player movement
  (:Pressed
    (Variables|Default|SetforwardAxis 1.0))
  (:Released
    (Variables|Default|SetforwardAxis 0.0)))

(event Input|KeyboardEvents|S
  (params (Key :type Key%20Structure))
  ;[1 0.2708 0.2708] Please don't do this in your final build. Always use 'Edit > Project Settings > Input' to set up action and axis mappings.
  ;;[1 1 1] Assigning keys for player movement
  (:Pressed
    (Variables|Default|SetforwardAxis -1.0))
  (:Released
    (Variables|Default|SetforwardAxis 0.0)))

(event Input|KeyboardEvents|A
  (params (Key :type Key%20Structure))
  ;[1 0.2708 0.2708] Please don't do this in your final build. Always use 'Edit > Project Settings > Input' to set up action and axis mappings.
  ;;[1 1 1] Assigning keys for player movement
  (:Pressed
    (Variables|Default|SetrightAxis -1.0))
  (:Released
    (Variables|Default|SetrightAxis 0.0)))

(event Input|KeyboardEvents|D
  (params (Key :type Key%20Structure))
  ;[1 0.2708 0.2708] Please don't do this in your final build. Always use 'Edit > Project Settings > Input' to set up action and axis mappings.
  ;;[1 1 1] Assigning keys for player movement
  (:Pressed
    (Variables|Default|SetrightAxis 1.0))
  (:Released
    (Variables|Default|SetrightAxis 0.0)))

(event Input|KeyboardEvents|SpaceBar
  (params (Key :type Key%20Structure))
  ;[1 0.2708 0.2708] Please don't do this in your final build. Always use 'Edit > Project Settings > Input' to set up action and axis mappings.
  ;;[1 1 1] Make player jump (Space Bar)
  (:Pressed
    (Character|Jump)))

(fn ConstructionScript)