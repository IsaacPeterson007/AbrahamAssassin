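; Physics-simulated arrow projectile that damages whatever it hits, then sticks or cleans itself up.
; On hit it attaches to the struck bone of an ArcherAIPawn (calling HitMe) or living TPPChar, with TPPChar hits destroyed shortly after.
; Actors or components tagged "Stickable" freeze it in place without collision.
; Other hits make Tick watch velocity until the arrow rests, then freeze it and destroy it after a delay.
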(event EventTick
  (params (DeltaSeconds :type Float%20%28single-precision%29))
  (bind _staticmesh (Variables|Default|GetStaticMesh))
  (bind _staticmesh_2 (Variables|Default|GetStaticMesh))
  ;[1 1 1] if we hit a non-stickable object, we start monitoring the velocity, once it hits 0, stop simulating physics, remove the collision and destroy the arrow after X seconds.
  (if (Variables|Default|GetwatchPhysics)
    (if (Physics|IsSimulatingPhysics _staticmesh "None")
      (if (<= (Math|Vector|VectorLength (Transformation|GetComponentVelocity _staticmesh)) 0.1)
        (Physics|SetSimulatePhysics _staticmesh_2 false)
        (Collision|SetCollisionEnabled _staticmesh_2 "NoCollision")
        (Utilities|FlowControl|Delay 3.0)
        (Actor|DestroyActor)))))

(event Collision|EventHit
  (params (MyComp :type Primitive%20Component%20Object%20Reference) (Other :type Actor%20Object%20Reference) (OtherComp :type Primitive%20Component%20Object%20Reference) (bSelfMoved :type Boolean) (HitLocation :type Vector :default "0, 0, 0") (HitNormal :type Vector :default "0, 0, 0") (NormalImpulse :type Vector :default "0, 0, 0") (Hit :type Hit%20Result%20Structure%20%28by%20ref%29))
  ;[1 1 1] if the arrow hit a stickable object, turn off simulating physics and make it static. Leave the arrow there for looks tho
  (Game|Damage|ApplyDamage Other 25.0 0 0)
  (Utilities|FlowControl|Sequence
    (:then_0
      (bind _asarcher_aipawn (Utilities|Casting|CastToArcherAIPawn Other)
        (:then
          (Default|HitMe _asarcher_aipawn Hit)
          (Transformation|AttachComponentToComponent (Variables|Default|GetStaticMesh) OtherComp (.HitBoneName (Collision|BreakHitResult Hit)) "SnapToTarget" "KeepRelative" "KeepRelative" true :!label _label)
          (Variables|Default|SetalreadyAppliedDamage true))
        (:CastFailed
          (bind _astppchar (Utilities|Casting|CastToTPPChar Other))
          (Utilities|FlowControl|Sequence
            (:then_0
              (if (not (Variables|/Game/Adams/Archer/Blueprints/TPPChar.TPPChar_C|GetisDead _astppchar))
                (goto _label)
                (else
                  _)))
            (:then_1
              (Utilities|FlowControl|Delay 1.0)))
          (Actor|DestroyActor))))
    (:then_1
      (if (Utilities|IsValid (Variables|Default|GetStaticMesh))
        (if (or (Actor|ActorHasTag Other "Stickable") (Components|ComponentHasTag OtherComp "Stickable"))
          (Physics|SetSimulatePhysics (Variables|Default|GetStaticMesh) false)
          (Collision|SetCollisionEnabled (Variables|Default|GetStaticMesh) "NoCollision")
          (Variables|Default|SetalreadyAppliedDamage true)
          (else
            (Variables|Default|SetwatchPhysics true)))))))

(fn ConstructionScript)