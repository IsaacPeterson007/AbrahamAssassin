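; Physics-driven arrow actor that reacts to what it hits, either sticking in place or settling and despawning.
; Hitting an AI_Archer_BP calls its HitMe and attaches the arrow mesh to the struck bone.
; Actors or components tagged Stickable freeze the arrow with collision off, leaving it in the world.
; Other hits make Tick watch velocity until nearly zero, then disable physics and collision and destroy the arrow after a delay.
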(event EventTick
  (params (DeltaSeconds :type Float%20%28single-precision%29))
  (bind _staticmesh (Variables|Default|GetStaticMesh))
  (bind _staticmesh_2 (Variables|Default|GetStaticMesh))
  ;[1 1 1] if we hit a non-stickable object, we start monitoring the velocity, once it hits 0, stop simulating physics, remove the collision and destroy the arrow after X seconds.
  (if (Variables|Default|GetwatchPhysics)
    (if (Physics|IsSimulatingPhysics _staticmesh "None")
      (if (<= (Math|Vector|VectorLength (Transformation|GetComponentVelocity _staticmesh)) 0.1)
        (Physics|SetSimulatePhysics _staticmesh_2 false)
        (Collision|SetCollisionEnabled _staticmesh_2 "NoCollision")
        (Utilities|FlowControl|Delay 3.0)
        (Actor|DestroyActor)))))

(event Collision|EventHit
  (params (MyComp :type Primitive%20Component%20Object%20Reference) (Other :type Actor%20Object%20Reference) (OtherComp :type Primitive%20Component%20Object%20Reference) (bSelfMoved :type Boolean) (HitLocation :type Vector :default "0, 0, 0") (HitNormal :type Vector :default "0, 0, 0") (NormalImpulse :type Vector :default "0, 0, 0") (Hit :type Hit%20Result%20Structure%20%28by%20ref%29))
  ;[1 1 1] if the arrow hit a stickable object, turn off simulating physics and make it static. Leave the arrow there for looks tho
  (Utilities|FlowControl|Sequence
    (:then_0
      (bind _asai_archer_bp (Utilities|Casting|CastToAI_Archer_BP Other))
      (Default|HitMe _asai_archer_bp Hit)
      (Transformation|AttachComponentToComponent (Variables|Default|GetStaticMesh) OtherComp (.HitBoneName (Collision|BreakHitResult Hit)) "SnapToTarget" "KeepRelative" "KeepRelative" true))
    (:then_1
      (if (or (Actor|ActorHasTag Other "Stickable") (Components|ComponentHasTag OtherComp "Stickable"))
        (Physics|SetSimulatePhysics (Variables|Default|GetStaticMesh) false)
        (Collision|SetCollisionEnabled (Variables|Default|GetStaticMesh) "NoCollision")
        (else
          (Variables|Default|SetwatchPhysics true))))))

(fn ConstructionScript)