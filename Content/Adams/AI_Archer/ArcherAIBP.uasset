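; Archer character Blueprint, named as an AI, with aiming and bow-shooting logic that is largely unwired.
; Its Hit event prints the mesh bone closest to the impact as debug output.
; Aim toggles walk speed, crosshair widget and lerp flags, while UpdateCrosshair projects a point ahead of the player onto the screen.
; Camera lerp loops and FireArrow's trace-and-impulse arrow spawn are disconnected, and nothing here calls these functions.
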(event Collision|EventHit
  (params (MyComp :type Primitive%20Component%20Object%20Reference) (Other :type Actor%20Object%20Reference) (OtherComp :type Primitive%20Component%20Object%20Reference) (bSelfMoved :type Boolean) (HitLocation :type Vector :default "0, 0, 0") (HitNormal :type Vector :default "0, 0, 0") (NormalImpulse :type Vector :default "0, 0, 0") (Hit :type Hit%20Result%20Structure%20%28by%20ref%29))
  (Development|PrintString (Utilities|String|ToString(Name) (.ReturnValue (Class|SkinnedMeshComponent|FindClosestBoneK2 (Variables|Character|GetMesh) (.Location (Collision|BreakHitResult Hit)) 0.0))))
  (Development|PrintString "Hello"))

(fn ConstructionScript)

(fn UpdateCrosshair
  (bind _returnvalue (Game|GetPlayerCharacter 0))
  (if (Variables|Default|GetisAiming)
    (Class|CanvasPanelSlot|SetPosition (Class|WidgetLayoutLibrary|SlotasCanvasSlot (Variables|/Game/Adams/Archer/CrosshairWidget.CrosshairWidget_C|GetImage_645 (Variables|Default|GetCrosshairWidget))) (.ScreenPosition (Class|WidgetLayoutLibrary|ProjectWorldLocationtoWidgetPosition (Game|GetPlayerController 0) (+ (Transformation|GetActorLocation _returnvalue) (* (Transformation|GetActorForwardVector _returnvalue) (LocalVariables|GetCenterDistance))))))))

(fn Aim
  (bind _charactermovement (Variables|Character|GetCharacterMovement))
  (bind _output_get (Variables|Default|SetisAiming (not (Variables|Default|GetisAiming))))
  (if _output_get
    (Variables|/Script/Engine.CharacterMovementComponent|SetMaxWalkSpeed _charactermovement (Variables|Default|GetwalkSpeedAiming))
    (bind _returnvalue (UserInterface|CreateWidget "/Game/Adams/Archer/CrosshairWidget.CrosshairWidget_C"))
    (bind _output_get_2 (Variables|Default|SetCrosshairWidget _returnvalue))
    (UserInterface|Viewport|AddtoViewport _output_get_2 0)
    (Variables|Default|SetlerpForward true)
    (else
      ;[1 1 1] unaim
      (Variables|/Script/Engine.CharacterMovementComponent|SetMaxWalkSpeed _charactermovement (Variables|Default|GetdefaultMaxSpeed))
      (if (not (Variables|Default|GetisAiming))
        (Widget|RemovefromParent (Variables|Default|GetCrosshairWidget))
        (Variables|Default|SetlerpBack true)))))

(fn FireArrow)