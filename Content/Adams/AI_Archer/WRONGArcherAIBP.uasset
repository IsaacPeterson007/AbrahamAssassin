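; Archer character Blueprint, named as an AI, that classifies hits by body region and carries player-style aiming logic.
; On Hit, it finds the closest mesh bone, maps it through bone lists to a region defaulting to Gut, and prints it.
; Aim toggles walk speed and crosshair, which UpdateCrosshair projects ahead of the player, but neither is called here.
; FireArrow is empty; its trace-and-spawn code and the camera lerp loops are disconnected.
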(event Collision|EventHit
  (params (MyComp :type Primitive%20Component%20Object%20Reference) (Other :type Actor%20Object%20Reference) (OtherComp :type Primitive%20Component%20Object%20Reference) (bSelfMoved :type Boolean) (HitLocation :type Vector :default "0, 0, 0") (HitNormal :type Vector :default "0, 0, 0") (NormalImpulse :type Vector :default "0, 0, 0") (Hit :type Hit%20Result%20Structure%20%28by%20ref%29))
  (bind _location (CallFunction|GetHitLocation (.ReturnValue (Class|SkinnedMeshComponent|FindClosestBoneK2 (Variables|Character|GetMesh) (.ImpactPoint (Collision|BreakHitResult Hit)) 0.0))))
  (Development|PrintString (Utilities|String|ToString(Name) _location)))

(fn ConstructionScript)

(fn UpdateCrosshair
  (bind _returnvalue (Game|GetPlayerCharacter 0))
  (if (Variables|Default|GetisAiming)
    (Class|CanvasPanelSlot|SetPosition (Class|WidgetLayoutLibrary|SlotasCanvasSlot (Variables|/Game/Adams/Archer/CrosshairWidget.CrosshairWidget_C|GetImage_645 (Variables|Default|GetCrosshairWidget))) (.ScreenPosition (Class|WidgetLayoutLibrary|ProjectWorldLocationtoWidgetPosition (Game|GetPlayerController 0) (+ (Transformation|GetActorLocation _returnvalue) (* (Transformation|GetActorForwardVector _returnvalue) (LocalVariables|GetCenterDistance))))))))

(fn Aim
  (bind _charactermovement (Variables|Character|GetCharacterMovement))
  (bind _output_get (Variables|Default|SetisAiming (not (Variables|Default|GetisAiming))))
  (if _output_get
    (Variables|/Script/Engine.CharacterMovementComponent|SetMaxWalkSpeed _charactermovement (Variables|Default|GetwalkSpeedAiming))
    (bind _returnvalue (UserInterface|CreateWidget "/Game/Adams/Archer/CrosshairWidget.CrosshairWidget_C"))
    (bind _output_get_2 (Variables|Default|SetCrosshairWidget _returnvalue))
    (UserInterface|Viewport|AddtoViewport _output_get_2 0)
    (Variables|Default|SetlerpForward true)
    (else
      ;[1 1 1] unaim
      (Variables|/Script/Engine.CharacterMovementComponent|SetMaxWalkSpeed _charactermovement (Variables|Default|GetdefaultMaxSpeed))
      (if (not (Variables|Default|GetisAiming))
        (Widget|RemovefromParent (Variables|Default|GetCrosshairWidget))
        (Variables|Default|SetlerpBack true)))))

(fn FireArrow)

(fn GetHitLocation
  (params (bone :type Name))
  (Utilities|FlowControl|Sequence
    (:then_0
      ;[1 1 1] Determine hit location from bone name
      (if (Utilities|Array|ContainsItem (LocalVariables|GetHeadBones) bone)
        (LocalVariables|SetHitBone "Head")
        (elif (Utilities|Array|ContainsItem (LocalVariables|GetChestBones) bone)
          (LocalVariables|SetHitBone "Chest")
          (elif (Utilities|Array|ContainsItem (LocalVariables|GetGutBones) bone)
            (LocalVariables|SetHitBone "Gut")
            (elif (Utilities|Array|ContainsItem (LocalVariables|GetLeftArmBones) bone)
              (LocalVariables|SetHitBone "LeftArm")
              (elif (Utilities|Array|ContainsItem (LocalVariables|GetRightArmBones) bone)
                (LocalVariables|SetHitBone "RightArm")
                (elif (Utilities|Array|ContainsItem (LocalVariables|GetLeftLegBones) bone)
                  (LocalVariables|SetHitBone "LeftLeg")
                  (elif (Utilities|Array|ContainsItem (LocalVariables|GetRightLegBones) bone)
                    (LocalVariables|SetHitBone "RightLeg")
                    (else
                      ;;[1 0.983 0.364] Default will be a gut shot
                      (LocalVariables|SetHitBone "Gut"))))))))))
    (:then_1
      (return (LocalVariables|GetHitBone)))))